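; Cartoon-material character base (BP_Character_2D) that feeds custom lighting parameters into its mesh materials.
; SETMSM turns cached mesh materials into dynamic instances stored in MTA and applies custom depth and stencil settings.
; Tick drives the lighting update, which uses BPLing to push A, B and C light channels to each instance, plus a Run channel after the loop.
; Construction configures capsule and movement, then calls Lig; a helper sets shadow color limits.
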(event Custom|获取材质
  (params (目标 :type Mesh%20Component%20Object%20Reference))
  (Utilities|Array|Clear (Variables|LigC|GetGet%20Mat_V))
  (CallFunction|GetMat 目标))

(event Custom|BP_Lig
  (for _array_element (Variables|基础设置|GetMTA)
    (Utilities|FlowControl|Sequence
      (:then_0
        (Default|LIGAMF (Variables|Default|GetBP_Ling) _array_element (Variables|LigA|GetLing%20Location%20A) (Variables|LigA|GetLing%20Toward%20A) (Variables|LigA|GetLing%20Color%20A) (Variables|LigA|GetRadius%20A) (Variables|LigA|GetHardness%20A) (Variables|LigA|GetPower%20A) (Variables|LigA|GetBool%20A) (Variables|LigA|GetKG%20A) (Variables|LigA|GetShadow%20Offer%20A)))
      (:then_1
        (Default|LIGBMF (Variables|Default|GetBP_Ling) _array_element (Variables|LigB|GetLing%20Location%20B) (Variables|LigB|GetLing%20Toward%20B) (Variables|LigB|GetLing%20Color%20B) (Variables|LigB|GetRadius%20B) (Variables|LigB|GetHardness%20B) (Variables|LigB|GetPower%20B) (Variables|LigB|GetBool%20B) (Variables|LigB|GetKG%20B) (Variables|LigB|GetShadow%20Offer%20B)))
      (:then_2
        (Default|LIGCMF (Variables|Default|GetBP_Ling) _array_element (Variables|LigC|GetLing%20Location%20C) (Variables|LigC|GetLing%20Toward%20C) (Variables|LigC|GetLing%20Color%20C) (Variables|LigC|GetRadius%20C) (Variables|LigC|GetHardness%20C) (Variables|LigC|GetPower%20C) (Variables|LigC|GetBool%20C) (Variables|LigC|GetKG%20C) (Variables|LigC|GetShadow%20Offer%20C)))))
  (Default|LIGRunMF (Variables|Default|GetBP_Ling) _array_element (Variables|Ling_Run|GetLing%20Location%20Run) (Variables|LingRun|GetLing%20Toward%20Run) (Variables|LingRun|GetLing%20Color%20Run) (Variables|LingRun|GetRadius%20Run) (Variables|LingRun|GetHardness%20Run) (Variables|LingRun|GetPower%20Run) (Variables|LingRun|GetBool%20Run) (Variables|LingRun|GetKG%20Run) (Variables|LingRun|GetShadow%20Offer%20Run)))

(event EventBeginPlay
  (Pawn|Components|CharacterMovement|SetMovementMode (Variables|Character|GetCharacterMovement) (Variables|基础设置|GetNew%20Movement%20Mode) 0))

(event Collision|EventActorBeginOverlap
  (params (OtherActor :type Actor%20Object%20Reference)))

(event EventTick
  (params (DeltaSeconds :type Float%20%28single-precision%29))
  (CallFunction|BpLig))

(fn ConstructionScript
  (bind _capsulecomponent (Variables|Collision|GetCapsuleComponent))
  (Collision|SetCollisionEnabled _capsulecomponent (Variables|基础设置|GetNew%20Type))
  (Components|Capsule|SetCapsuleHalfHeight _capsulecomponent (Variables|基础设置|GetHalf%20Height) true)
  (Components|Capsule|SetCapsuleRadius _capsulecomponent (Variables|基础设置|GetRadius) true)
  (Pawn|Components|CharacterMovement|SetMovementMode (Variables|Character|GetCharacterMovement) (Variables|基础设置|GetNew%20Movement%20Mode) 0)
  (CallFunction|Lig))

(fn SETMSM
  (params (MS :type Mesh%20Component%20Object%20Reference) (SK :type Mesh%20Component%20Object%20Reference))
  (Utilities|FlowControl|Sequence
    (:then_0
      (if (Utilities|IsValid MS)
        (Default|SKMater (Variables|Default|GetBP_Ling) SK)
        (CallFunction|获取材质)
        (for _array_element (Rendering|Material|GetMaterials SK)
          _)))
    (:then_1
      (if (Utilities|IsValid SK)
        (if (> (Utilities|Array|Length (Variables|LigC|GetGet%20Mat_V)) 0)
          (Utilities|Array|Clear (Variables|基础设置|GetMTA))
          (for (_array_element_2 _array_index) (Variables|LigC|GetGet%20Mat_V)
            (bind _returnvalue (Rendering|Material|CreateDynamicMaterialInstance _array_element_2 (Utilities|String|StringToName (Utilities|String|Append (Utilities|GetObjectName SK) (Utilities|String|ToString(Integer) _array_index))) "None" :!class /Script/Engine.KismetMaterialLibrary))
            (Utilities|Array|Add (Variables|基础设置|GetMTA) _returnvalue)
            (Rendering|Material|SetMaterial SK _array_index _returnvalue))
          (else
            (CallFunction|获取材质 SK)))))
    (:then_2
      (Utilities|FlowControl|Sequence
        (:then_0
          (if (Utilities|IsValid MS)
            (Rendering|SetRenderCustomDepth MS (Variables|基础设置|Get设置自定义深度))
            (Rendering|SetCustomDepthStencilValue MS (Variables|基础设置|Get设置自定义深度值))))
        (:then_1
          (if (Utilities|IsValid SK)
            (Rendering|SetRenderCustomDepth SK (Variables|基础设置|Get设置自定义深度))
            (Rendering|SetCustomDepthStencilValue SK (Variables|基础设置|Get设置自定义深度值))))))))

(fn SetMatShadowColor
  (for _array_element (Variables|基础设置|GetMTA)
    (Rendering|Material|SetVectorParameterValue _array_element "Shadow_MAX" (Variables|基础设置|GetShadow_MAX) :!class /Script/Engine.MaterialInstanceDynamic)
    (Rendering|Material|SetVectorParameterValue _array_element "Shadow_MIN" (Variables|基础设置|GetShadow_MIN) :!class /Script/Engine.MaterialInstanceDynamic)))

(fn GetMat
  (params (目标 :type Mesh%20Component%20Object%20Reference))
  (Variables|LigC|SetGet%20Mat_V (Rendering|Material|GetMaterials 目标)))