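; BP_CarToon is a helper Blueprint for cartoon materials that feeds custom light data into material parameters.
; Five parallel functions serve light slots A, B, C, D and Run, each writing location, direction, color, falloff, power, switch and shadow-offset values to a given material.
; SK_Mater replaces a mesh's materials with transient dynamic instances so they can accept runtime changes.
; The event graph is empty, and nothing here calls these functions.
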(event EventBeginPlay)

(event EventTick
  (params (DeltaSeconds :type Float%20%28single-precision%29)))

(fn LIGAMF
  (params (M :type Material%20Instance%20Dynamic%20Object%20Reference) (Ling_Location_A :type Vector) (Ling_Toward_A :type Vector) (Ling_Color_A :type Linear%20Color%20Structure) (Radius_A :type Float%20%28single-precision%29) (Hardness_A :type Float%20%28single-precision%29) (Power_A :type Float%20%28single-precision%29) (Bool_A :type Float%20%28single-precision%29) (KG_A :type Float%20%28single-precision%29) (ShadowOffer_A :type Float%20%28single-precision%29))
  (if (Utilities|IsValid M)
    (Rendering|Material|SetVectorParameterValue M "Ling_Location_A" (Math|Conversions|ToLinearColor(Vector) Ling_Location_A) :!class /Script/Engine.MaterialInstanceDynamic)
    (Rendering|Material|SetVectorParameterValue M "Ling_Toward_A" (Math|Conversions|ToLinearColor(Vector) Ling_Toward_A) :!class /Script/Engine.MaterialInstanceDynamic)
    (Rendering|Material|SetVectorParameterValue M "Ling_Color_A" Ling_Color_A :!class /Script/Engine.MaterialInstanceDynamic)
    (Rendering|Material|SetScalarParameterValue M "Radius_A" Radius_A :!class /Script/Engine.MaterialInstanceDynamic)
    (Rendering|Material|SetScalarParameterValue M "Hardness_A" Hardness_A :!class /Script/Engine.MaterialInstanceDynamic)
    (Rendering|Material|SetScalarParameterValue M "Power_A" Power_A :!class /Script/Engine.MaterialInstanceDynamic)
    (Rendering|Material|SetScalarParameterValue M "Bool_A" Bool_A :!class /Script/Engine.MaterialInstanceDynamic)
    (Rendering|Material|SetScalarParameterValue M "KG_A" KG_A :!class /Script/Engine.MaterialInstanceDynamic)
    (Rendering|Material|SetScalarParameterValue M "ShadowOffer_A" ShadowOffer_A :!class /Script/Engine.MaterialInstanceDynamic)))

(fn LIGBMF
  (params (M :type Material%20Instance%20Dynamic%20Object%20Reference) (Ling_Location_B :type Vector) (Ling_Toward_B :type Vector) (Ling_Color_B :type Linear%20Color%20Structure) (Radius_B :type Float%20%28single-precision%29) (Hardness_B :type Float%20%28single-precision%29) (Power_B :type Float%20%28single-precision%29) (Bool_B :type Float%20%28single-precision%29) (KG_B :type Float%20%28single-precision%29) (ShadowOffer_B :type Float%20%28single-precision%29))
  (if (Utilities|IsValid M)
    (Rendering|Material|SetVectorParameterValue M "Ling_Location_B" (Math|Conversions|ToLinearColor(Vector) Ling_Location_B) :!class /Script/Engine.MaterialInstanceDynamic)
    (Rendering|Material|SetVectorParameterValue M "Ling_Toward_B" (Math|Conversions|ToLinearColor(Vector) Ling_Toward_B) :!class /Script/Engine.MaterialInstanceDynamic)
    (Rendering|Material|SetVectorParameterValue M "Ling_Color_B" Ling_Color_B :!class /Script/Engine.MaterialInstanceDynamic)
    (Rendering|Material|SetScalarParameterValue M "Radius_B" Radius_B :!class /Script/Engine.MaterialInstanceDynamic)
    (Rendering|Material|SetScalarParameterValue M "Hardness_B" Hardness_B :!class /Script/Engine.MaterialInstanceDynamic)
    (Rendering|Material|SetScalarParameterValue M "Power_B" Power_B :!class /Script/Engine.MaterialInstanceDynamic)
    (Rendering|Material|SetScalarParameterValue M "Bool_B" Bool_B :!class /Script/Engine.MaterialInstanceDynamic)
    (Rendering|Material|SetScalarParameterValue M "KG_B" KG_B :!class /Script/Engine.MaterialInstanceDynamic)
    (Rendering|Material|SetScalarParameterValue M "ShadowOffer_B" ShadowOffer_B :!class /Script/Engine.MaterialInstanceDynamic)))

(fn LIGCMF
  (params (M :type Material%20Instance%20Dynamic%20Object%20Reference) (Ling_Location_C :type Vector) (Ling_Toward_C :type Vector) (Ling_Color_C :type Linear%20Color%20Structure) (Radius_C :type Float%20%28single-precision%29) (Hardness_C :type Float%20%28single-precision%29) (Power_C :type Float%20%28single-precision%29) (Bool_C :type Float%20%28single-precision%29) (KG_C :type Float%20%28single-precision%29) (ShadowOffer_C :type Float%20%28single-precision%29))
  (if (Utilities|IsValid M)
    (Rendering|Material|SetVectorParameterValue M "Ling_Location_C" (Math|Conversions|ToLinearColor(Vector) Ling_Location_C) :!class /Script/Engine.MaterialInstanceDynamic)
    (Rendering|Material|SetVectorParameterValue M "Ling_Toward_C" (Math|Conversions|ToLinearColor(Vector) Ling_Toward_C) :!class /Script/Engine.MaterialInstanceDynamic)
    (Rendering|Material|SetVectorParameterValue M "Ling_Color_C" Ling_Color_C :!class /Script/Engine.MaterialInstanceDynamic)
    (Rendering|Material|SetScalarParameterValue M "Radius_C" Radius_C :!class /Script/Engine.MaterialInstanceDynamic)
    (Rendering|Material|SetScalarParameterValue M "Hardness_C" Hardness_C :!class /Script/Engine.MaterialInstanceDynamic)
    (Rendering|Material|SetScalarParameterValue M "Power_C" Power_C :!class /Script/Engine.MaterialInstanceDynamic)
    (Rendering|Material|SetScalarParameterValue M "Bool_C" Bool_C :!class /Script/Engine.MaterialInstanceDynamic)
    (Rendering|Material|SetScalarParameterValue M "KG_C" KG_C :!class /Script/Engine.MaterialInstanceDynamic)
    (Rendering|Material|SetScalarParameterValue M "ShadowOffer_C" ShadowOffer_C :!class /Script/Engine.MaterialInstanceDynamic)))

(fn LIGDMF
  (params (M :type Material%20Instance%20Dynamic%20Object%20Reference) (Ling_Location_D :type Vector) (Ling_Toward_D :type Vector) (Ling_Color_D :type Linear%20Color%20Structure) (Radius_D :type Float%20%28single-precision%29) (Hardness_D :type Float%20%28single-precision%29) (Power_D :type Float%20%28single-precision%29) (Bool_D :type Float%20%28single-precision%29) (KG_D :type Float%20%28single-precision%29) (ShadowOffer_D :type Float%20%28single-precision%29))
  (if (Utilities|IsValid M)
    (Rendering|Material|SetVectorParameterValue M "Ling_Location_D" (Math|Conversions|ToLinearColor(Vector) Ling_Location_D) :!class /Script/Engine.MaterialInstanceDynamic)
    (Rendering|Material|SetVectorParameterValue M "Ling_Toward_D" (Math|Conversions|ToLinearColor(Vector) Ling_Toward_D) :!class /Script/Engine.MaterialInstanceDynamic)
    (Rendering|Material|SetVectorParameterValue M "Ling_Color_D" Ling_Color_D :!class /Script/Engine.MaterialInstanceDynamic)
    (Rendering|Material|SetScalarParameterValue M "Radius_D" Radius_D :!class /Script/Engine.MaterialInstanceDynamic)
    (Rendering|Material|SetScalarParameterValue M "Hardness_D" Hardness_D :!class /Script/Engine.MaterialInstanceDynamic)
    (Rendering|Material|SetScalarParameterValue M "Power_D" Power_D :!class /Script/Engine.MaterialInstanceDynamic)
    (Rendering|Material|SetScalarParameterValue M "Bool_D" Bool_D :!class /Script/Engine.MaterialInstanceDynamic)
    (Rendering|Material|SetScalarParameterValue M "KG_D" KG_D :!class /Script/Engine.MaterialInstanceDynamic)
    (Rendering|Material|SetScalarParameterValue M "ShadowOffer_D" ShadowOffer_D :!class /Script/Engine.MaterialInstanceDynamic)))

(fn LIGRunMF
  (params (M :type Material%20Instance%20Dynamic%20Object%20Reference) (Ling_Location_Run :type Vector) (Ling_Toward_Run :type Vector) (Ling_Color_Run :type Linear%20Color%20Structure) (Radius_Run :type Float%20%28single-precision%29) (Hardness_Run :type Float%20%28single-precision%29) (Power_Run :type Float%20%28single-precision%29) (Bool_Run :type Float%20%28single-precision%29) (KG_Run :type Float%20%28single-precision%29) (ShadowOffer_Run :type Float%20%28single-precision%29))
  (if (Utilities|IsValid M)
    (Rendering|Material|SetVectorParameterValue M "Ling_Location_Run" (Math|Conversions|ToLinearColor(Vector) Ling_Location_Run) :!class /Script/Engine.MaterialInstanceDynamic)
    (Rendering|Material|SetVectorParameterValue M "Ling_Toward_Run" (Math|Conversions|ToLinearColor(Vector) Ling_Toward_Run) :!class /Script/Engine.MaterialInstanceDynamic)
    (Rendering|Material|SetVectorParameterValue M "Ling_Color_Run" Ling_Color_Run :!class /Script/Engine.MaterialInstanceDynamic)
    (Rendering|Material|SetScalarParameterValue M "Radius_Run" Radius_Run :!class /Script/Engine.MaterialInstanceDynamic)
    (Rendering|Material|SetScalarParameterValue M "Hardness_Run" Hardness_Run :!class /Script/Engine.MaterialInstanceDynamic)
    (Rendering|Material|SetScalarParameterValue M "Power_Run" Power_Run :!class /Script/Engine.MaterialInstanceDynamic)
    (Rendering|Material|SetScalarParameterValue M "Bool_Run" Bool_Run :!class /Script/Engine.MaterialInstanceDynamic)
    (Rendering|Material|SetScalarParameterValue M "KG_Run" KG_Run :!class /Script/Engine.MaterialInstanceDynamic)
    (Rendering|Material|SetScalarParameterValue M "ShadowOffer_Run" ShadowOffer_Run :!class /Script/Engine.MaterialInstanceDynamic)))

(fn SKMater
  (params (Mater :type Primitive%20Component%20Object%20Reference))
  (for _index (range 0 (Rendering|Material|GetNumMaterials Mater))
    (bind _returnvalue (Rendering|Material|CreateDynamicMaterialInstance (Rendering|Material|GetMaterial Mater _index) (Utilities|String|StringToName (Utilities|GetObjectName Mater)) "Transient" :!class /Script/Engine.KismetMaterialLibrary))
    (Rendering|Material|SetMaterial Mater _index _returnvalue))
  (return))