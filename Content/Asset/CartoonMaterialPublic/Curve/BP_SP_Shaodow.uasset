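; Actor Blueprint that defines a spherical zone for the cartoon materials, apparently to control their shadowing.
; Its construction script calls UP, which writes the actor location, radius, hardness, min/max and shadow color limits into the MP_Cartoon material parameter collection.
; UP also resizes the Sphere component to match the radius.
; BeginPlay, Tick and overlap events are empty, so nothing updates the values during play.
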(event Custom|UP
  (Rendering|Material|SetVectorParameterValue "/Game/Asset/CartoonMaterialPublic/Curve/MP_Cartoon.MP_Cartoon" "Location" (Math|Conversions|ToLinearColor(Vector) (Transformation|GetActorLocation)) :!class /Script/Engine.KismetMaterialLibrary)
  (Rendering|Material|SetScalarParameterValue "/Game/Asset/CartoonMaterialPublic/Curve/MP_Cartoon.MP_Cartoon" "Radius" (Variables|Default|GetRadius) :!class /Script/Engine.KismetMaterialLibrary)
  (Rendering|Material|SetScalarParameterValue "/Game/Asset/CartoonMaterialPublic/Curve/MP_Cartoon.MP_Cartoon" "Hardness" (Variables|Default|GetHardness) :!class /Script/Engine.KismetMaterialLibrary)
  (Rendering|Material|SetScalarParameterValue "/Game/Asset/CartoonMaterialPublic/Curve/MP_Cartoon.MP_Cartoon" "Max" (Variables|Default|GetMax) :!class /Script/Engine.KismetMaterialLibrary)
  (Rendering|Material|SetScalarParameterValue "/Game/Asset/CartoonMaterialPublic/Curve/MP_Cartoon.MP_Cartoon" "Min" (Variables|Default|GetMin) :!class /Script/Engine.KismetMaterialLibrary)
  (Rendering|Material|SetScalarParameterValue "/Game/Asset/CartoonMaterialPublic/Curve/MP_Cartoon.MP_Cartoon" "Shadow_Max_Color_Max" (Variables|Default|GetShadow_Max_Color_Max) :!class /Script/Engine.KismetMaterialLibrary)
  (Rendering|Material|SetScalarParameterValue "/Game/Asset/CartoonMaterialPublic/Curve/MP_Cartoon.MP_Cartoon" "Shadow_Max_Color_Min" (Variables|Default|GetShadow_Max_Color_Min) :!class /Script/Engine.KismetMaterialLibrary)
  (Components|Sphere|SetSphereRadius (Variables|Default|GetSphere) (Variables|Default|GetRadius) true))

(event EventBeginPlay)

(event Collision|EventActorBeginOverlap
  (params (OtherActor :type Actor%20Object%20Reference)))

(event EventTick
  (params (DeltaSeconds :type Float%20%28single-precision%29)))

(fn ConstructionScript
  (CallFunction|UP))