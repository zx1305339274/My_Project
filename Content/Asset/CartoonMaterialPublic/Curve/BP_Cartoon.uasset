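; Actor Blueprint that feeds forward and up direction vectors to cartoon materials through the MP_SDFvalue parameter collection, likely for SDF-based shading.
; The normalized world-space offsets from Scene to the CustomMeshF and CustomMeshU marker components become the F and U vector parameters.
; The update runs in the construction script, on BeginPlay and every Tick, keeping the vectors in step with the components' transforms.
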(event Custom|UP
  (bind _scene (Variables|Default|GetScene))
  (bind _returnvalue (Transformation|GetWorldLocation _scene))
  (Rendering|Material|SetVectorParameterValue "/Game/Asset/CartoonMaterialPublic/Curve/MP_SDFvalue.MP_SDFvalue" "F" (Math|Conversions|ToLinearColor(Vector) (Math|Vector|Normalize (- (Transformation|GetWorldLocation (Variables|Default|GetCustomMeshF)) _returnvalue))) :!class /Script/Engine.KismetMaterialLibrary)
  (Rendering|Material|SetVectorParameterValue "/Game/Asset/CartoonMaterialPublic/Curve/MP_SDFvalue.MP_SDFvalue" "U" (Math|Conversions|ToLinearColor(Vector) (Math|Vector|Normalize (- (Transformation|GetWorldLocation (Variables|Default|GetCustomMeshU)) _returnvalue))) :!class /Script/Engine.KismetMaterialLibrary))

(event EventBeginPlay
  (bind _scene (Variables|Default|GetScene))
  (bind _returnvalue (Transformation|GetWorldLocation _scene))
  (Rendering|Material|SetVectorParameterValue "/Game/Asset/CartoonMaterialPublic/Curve/MP_SDFvalue.MP_SDFvalue" "F" (Math|Conversions|ToLinearColor(Vector) (Math|Vector|Normalize (- (Transformation|GetWorldLocation (Variables|Default|GetCustomMeshF)) _returnvalue))) :!class /Script/Engine.KismetMaterialLibrary)
  (Rendering|Material|SetVectorParameterValue "/Game/Asset/CartoonMaterialPublic/Curve/MP_SDFvalue.MP_SDFvalue" "U" (Math|Conversions|ToLinearColor(Vector) (Math|Vector|Normalize (- (Transformation|GetWorldLocation (Variables|Default|GetCustomMeshU)) _returnvalue))) :!class /Script/Engine.KismetMaterialLibrary))

(event Collision|EventActorBeginOverlap
  (params (OtherActor :type Actor%20Object%20Reference)))

(event EventTick
  (params (DeltaSeconds :type Float%20%28single-precision%29))
  (bind _scene (Variables|Default|GetScene))
  (bind _returnvalue (Transformation|GetWorldLocation _scene))
  (Rendering|Material|SetVectorParameterValue "/Game/Asset/CartoonMaterialPublic/Curve/MP_SDFvalue.MP_SDFvalue" "F" (Math|Conversions|ToLinearColor(Vector) (Math|Vector|Normalize (- (Transformation|GetWorldLocation (Variables|Default|GetCustomMeshF)) _returnvalue))) :!class /Script/Engine.KismetMaterialLibrary)
  (Rendering|Material|SetVectorParameterValue "/Game/Asset/CartoonMaterialPublic/Curve/MP_SDFvalue.MP_SDFvalue" "U" (Math|Conversions|ToLinearColor(Vector) (Math|Vector|Normalize (- (Transformation|GetWorldLocation (Variables|Default|GetCustomMeshU)) _returnvalue))) :!class /Script/Engine.KismetMaterialLibrary))

(fn ConstructionScript
  (CallFunction|UP))